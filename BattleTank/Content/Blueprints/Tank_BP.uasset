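; Player-controllable tank Blueprint that wires input to movement, aiming and firing components.
; On BeginPlay it initialises TankMovement with both tracks and TankAiming with the turret and barrel.
; Aim axes rotate the azimuth gimbal and spring arm, scaled by delta time, to orbit the camera.
; Move and track-throttle axes pass intents to TankMovement, while Fire calls TankAiming.
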(event `self.ReceiveBeginPlay`
  (`|ExecutionSequence`
    (:`then_0`
      (`TankMovementComponent.Initialise` (`self.TankMovement`) (`self.TankTrackLeft`) (`self.TankTrackRight`)))
    (:`then_1`
      (`TankAimingComponent.Initialise` (`self.TankAiming`) (`self.TankTurret`) (`self.TankBarrel`)))))

(event `InputAxis|AimAzimuth`
  (params (AxisValue :type "Float (single-precision)"))
  ;[1 1 1] Camera Input Binding
  (`SceneComponent.K2_AddLocalRotation` (`self.Azimuth Gimbal`) (`KismetMathLibrary.MakeRotator` 0.0 0.0 (* AxisValue (`GameplayStatics.GetWorldDeltaSeconds`) 100.0)) false false))

(event `InputAxis|AimElevation`
  (params (AxisValue :type "Float (single-precision)"))
  ;[1 1 1] Camera Input Binding
  (`SceneComponent.K2_AddLocalRotation` (`self.SpringArm`) (`KismetMathLibrary.MakeRotator` 0.0 (* AxisValue (`GameplayStatics.GetWorldDeltaSeconds`) 100.0)) false false))

(event `InputAction|Fire`
  (params (Key :type "Key Structure"))
  (:`Pressed`
    (`TankAimingComponent.Fire` (`self.TankAiming`))))

(event `InputAxis|MoveForward`
  (params (AxisValue :type "Float (single-precision)"))
  ;[1 1 1] Movement Components
  (`TankMovementComponent.IntendMoveForward` (`self.TankMovement`) AxisValue))

(event `InputAxis|MoveBackward`
  (params (AxisValue :type "Float (single-precision)"))
  ;[1 1 1] Movement Components
  (`TankMovementComponent.IntendMoveBackward` (`self.TankMovement`) AxisValue))

(event `InputAxis|RightTrackThrottle`
  (params (AxisValue :type "Float (single-precision)"))
  ;[1 1 1] Movement Components
  (`TankMovementComponent.IntendMoveRight` (`self.TankMovement`) AxisValue))

(event `InputAxis|LeftTrackThrottle`
  (params (AxisValue :type "Float (single-precision)"))
  ;[1 1 1] Movement Components
  (`TankMovementComponent.IntendMoveLeft` (`self.TankMovement`) AxisValue))

(fn `UserConstructionScript`)